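; BP_Pawn is a pawn that drives a scan effect from the IA_Scan Enhanced Input action.
; When the action starts or completes, it looks up the BP_Scan_AC component on its controller and calls StartScan or EndScan.
; Validity checks guard the controller and component, and each call prints a debug string.
; The pawn only forwards input, leaving the scan logic to that component.
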(event `EnhancedInput|/Game/ART/FX/ScanEffect/IA_Scan`
  (params (ActionValue :type Boolean) (ElapsedSeconds :type "Float (double-precision)") (TriggeredSeconds :type "Float (double-precision)") (InputAction :type "InputAction Object Reference" :default "/Game/ART/FX/ScanEffect/IA_Scan.IA_Scan"))
  (bind _returnvalue (`self.GetController`))
  (bind _returnvalue_2 (`self.GetController`))
  (bind _returnvalue_3 (`self.GetComponentByClass` _returnvalue "/Game/ART/FX/ScanEffect/BP_Scan_AC.BP_Scan_AC_C"))
  (bind _returnvalue_4 (`self.GetComponentByClass` _returnvalue_2 "/Game/ART/FX/ScanEffect/BP_Scan_AC.BP_Scan_AC_C"))
  (:`Started`
    (`/Engine/EditorBlueprintResources/StandardMacros.IsValid` _returnvalue_2
      (:`Is Valid`
        (`/Engine/EditorBlueprintResources/StandardMacros.IsValid` _returnvalue_4
          (:`Is Valid`
            (`/Game/ART/FX/ScanEffect/BP_Scan_AC.StartScan` _returnvalue_4)
            (`KismetSystemLibrary.PrintString` "Start Scan"))))))
  (:`Completed`
    (`/Engine/EditorBlueprintResources/StandardMacros.IsValid` _returnvalue
      (:`Is Valid`
        (`/Engine/EditorBlueprintResources/StandardMacros.IsValid` _returnvalue_3
          (:`Is Valid`
            (`/Game/ART/FX/ScanEffect/BP_Scan_AC.EndScan` _returnvalue_3)
            (`KismetSystemLibrary.PrintString` "End Scan")))))))

(fn `UserConstructionScript`)