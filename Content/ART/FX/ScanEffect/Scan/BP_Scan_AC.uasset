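; Player controller component that runs a fading scan post-process effect, toggled by StartScan and EndScan.
; A five-state machine advances normalized time on Tick, switching Tick off when faded out or invalid.
; It feeds time, state flags, grid size, range and controlled pawn location into MPC_Scan.
; A lazily spawned BP_Scan_Actor hosts the dynamic post-process material, its blend weight following an optional curve, and is optionally destroyed after fade-out.
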(event `self.ReceiveBeginPlay`
  (bind _asplayer_controller (cast `PlayerController` (`self.GetOwner`))
    (:`then`
      (set `self.PlayerController` _asplayer_controller)
      (`self.UpdateScanState` "NewEnumerator3" true)
      (`KismetMaterialLibrary.SetScalarParameterValue` "/Game/ART/FX/ScanEffect/Scan/Material/MPC_Scan.MPC_Scan" "GridCellSize" (`self.GridCellSize`))
      (`KismetMaterialLibrary.SetScalarParameterValue` "/Game/ART/FX/ScanEffect/Scan/Material/MPC_Scan.MPC_Scan" "Range" (`self.Range`)))
    (:`CastFailed`
      (`self.UpdateScanState` "NewEnumerator4" true))))

(event `self.ReceiveTick`
  (params (DeltaSeconds :type "Float (single-precision)"))
  (bind _playercontroller (`self.PlayerController`))
  (bind _returnvalue (`Controller.K2_GetPawn` _playercontroller))
  (`self.UpdateScanTime` DeltaSeconds)
  (switch `/Game/ART/FX/ScanEffect/Scan/Other/EBP_Scan_State` (`self.GetScanState`)
    (:`NewEnumerator0`
      (`self.Update Scan PPBlend Weight` :!label _label))
    (:`NewEnumerator1`
      _)
    (:`NewEnumerator2`
      (goto _label))
    (:`NewEnumerator3`
      _))
  (`/Engine/EditorBlueprintResources/StandardMacros.IsValid` _playercontroller
    (:`Is Valid`
      (`/Engine/EditorBlueprintResources/StandardMacros.IsValid` _returnvalue
        (:`Is Valid`
          (`KismetMaterialLibrary.SetVectorParameterValue` "/Game/ART/FX/ScanEffect/Scan/Material/MPC_Scan.MPC_Scan" "Location" (`KismetMathLibrary.Conv_VectorToLinearColor` (`Actor.K2_GetActorLocation` _returnvalue))))))))

(fn `DestroyScanPPActor`
  (bind _scan_actor (`self.Scan Actor`))
  (if (and (`KismetSystemLibrary.IsValid` _scan_actor) (`self.bDestroyActor`))
    (`Actor.K2_DestroyActor` _scan_actor)
    (set `self.Scan Actor` null)))

(fn `EndScan`
  (returns (bEnded :type Boolean))
  (switch `/Game/ART/FX/ScanEffect/Scan/Other/EBP_Scan_State` (`self.GetScanState`)
    (:`NewEnumerator0`
      _)
    (:`NewEnumerator1`
      _)
    (:`NewEnumerator2`
      (return false))
    (:`NewEnumerator3`
      (return false))
    (:`NewEnumerator4`
      (return false)))
  (bind _bupdated (`self.UpdateScanState` "NewEnumerator2"))
  (return _bupdated))

(fn `GetScanPPActor`
  (returns (ScanActor :type "/Game/ART/FX/ScanEffect/Scan/BP_Scan_Actor Object Reference"))
  (bind _scan_actor (`self.Scan Actor`))
  (bind _ppmaterial (`self.PPmaterial`))
  (bind _postprocess (`/Game/ART/FX/ScanEffect/Scan/BP_Scan_Actor.PostProcess` (`self.Scan Actor`)))
  (`/Engine/EditorBlueprintResources/StandardMacros.IsValid` _scan_actor
    (:`Is Valid`
      (return _scan_actor))
    (:`Is Not Valid`
      (bind _returnvalue (`|SpawnActorFromClass` "/Game/ART/FX/ScanEffect/Scan/BP_Scan_Actor.BP_Scan_Actor_C" (`KismetMathLibrary.MakeTransform` (0.0 0.0 0.0)) "Undefined" "MultiplyWithRoot" null null))
      (set `self.Scan Actor` _returnvalue)
      (`|ExecutionSequence`
        (:`then_0`
          (`/Engine/EditorBlueprintResources/StandardMacros.IsValid` (`self.PPmid`)
            (:`Is Valid`
              _)
            (:`Is Not Valid`
              (`/Engine/EditorBlueprintResources/StandardMacros.IsValid` _ppmaterial
                (:`Is Valid`
                  (bind _returnvalue_2 (`KismetMaterialLibrary.CreateDynamicMaterialInstance` _ppmaterial))
                  (set `self.PPmid` _returnvalue_2)))))
          (`/Engine/EditorBlueprintResources/StandardMacros.IsValid` _postprocess
            (:`Is Valid`
              (setmembers `PostProcessSettings` :`StructRef` (`PostProcessComponent.Settings` _postprocess) :`WeightedBlendables` (make `WeightedBlendables` (`|MakeArray` (make `WeightedBlendable` 1.0 (`self.PPmid`))))))))
        (:`then_1`
          (return _scan_actor))))))

(fn `GetScanState`
  (returns (State :type "/Game/ART/FX/ScanEffect/Scan/Other/EBP_Scan_State Enum"))
  (return (`self.State`)))

(fn `StartScan`
  (returns (bStarted :type Boolean))
  (switch `/Game/ART/FX/ScanEffect/Scan/Other/EBP_Scan_State` (`self.GetScanState`)
    (:`NewEnumerator0`
      _)
    (:`NewEnumerator1`
      _)
    (:`NewEnumerator2`
      (bind _bupdated (`self.UpdateScanState` "NewEnumerator0" :!label _label))
      (return _bupdated))
    (:`NewEnumerator3`
      (goto _label))
    (:`NewEnumerator4`
      _))
  (return false))

(fn `Update Scan PPBlend Weight`
  (locals (ThisTime :type "Float (single-precision)" :default 0.0))
  (bind _ppblendcurve (`self.PPBlendCurve`))
  (bind _scannormalizedtime (`self.ScanNormalizedTime`))
  (`/Engine/EditorBlueprintResources/StandardMacros.IsValid` _ppblendcurve
    (:`Is Valid`
      (set `local.ThisTime` (`CurveFloat.GetFloatValue` _ppblendcurve _scannormalizedtime)))
    (:`Is Not Valid`
      (set `local.ThisTime` _scannormalizedtime)))
  (bind _scanactor (`self.GetScanPPActor`))
  (`/Engine/EditorBlueprintResources/StandardMacros.IsValid` _scanactor
    (:`Is Valid`
      (bind _postprocess (`/Game/ART/FX/ScanEffect/Scan/BP_Scan_Actor.PostProcess` _scanactor))
      (`/Engine/EditorBlueprintResources/StandardMacros.IsValid` _postprocess
        (:`Is Valid`
          (set `PostProcessComponent.BlendWeight` (`local.ThisTime`) _postprocess))))))

(fn `UpdateScanState`
  (params (State :type "/Game/ART/FX/ScanEffect/Scan/Other/EBP_Scan_State Enum" :default "NewEnumerator0") (bForce :type Boolean))
  (returns (bUpdated :type Boolean))
  (if (or bForce (`|EnumInequality` State (`self.State`)))
    (`|ExecutionSequence`
      (:`then_0`
        (switch `/Game/ART/FX/ScanEffect/Scan/Other/EBP_Scan_State` (`self.State`) ; Exit current state
          (:`NewEnumerator1`
            (`KismetMaterialLibrary.SetScalarParameterValue` "/Game/ART/FX/ScanEffect/Scan/Material/MPC_Scan.MPC_Scan" "bFadedIN" 0.0))
          (:`NewEnumerator3`
            (`KismetMaterialLibrary.SetScalarParameterValue` "/Game/ART/FX/ScanEffect/Scan/Material/MPC_Scan.MPC_Scan" "bFadedOUT" 0.0)
            (`self.SetComponentTickEnabled` true))))
      (:`then_1`
        (bind _output_get (set `self.State` State))
        (switch `/Game/ART/FX/ScanEffect/Scan/Other/EBP_Scan_State` _output_get ; Enter new state
          (:`NewEnumerator1`
            (`KismetMaterialLibrary.SetScalarParameterValue` "/Game/ART/FX/ScanEffect/Scan/Material/MPC_Scan.MPC_Scan" "bFadedIN" 1.0)
            (`self.Update Scan PPBlend Weight`))
          (:`NewEnumerator3`
            (`KismetMaterialLibrary.SetScalarParameterValue` "/Game/ART/FX/ScanEffect/Scan/Material/MPC_Scan.MPC_Scan" "bFadedOUT" 1.0)
            (`self.Update Scan PPBlend Weight`)
            (`self.SetComponentTickEnabled` false :!label _label)
            (`self.DestroyScanPPActor`))
          (:`NewEnumerator4`
            (goto _label))))
      (:`then_2`
        (return true)))
    (else
      (return false))))

(fn `UpdateScanTime`
  (params (DeltaTime :type "Float (double-precision)"))
  (returns (bUpdated :type Boolean))
  (`|ExecutionSequence`
    (:`then_0`
      (switch `/Game/ART/FX/ScanEffect/Scan/Other/EBP_Scan_State` (`self.GetScanState`)
        (:`NewEnumerator0`
          (bind _output_get (set `self.ScanNormalizedTime` (+ (`self.ScanNormalizedTime`) (* (`local.DeltaTime`) (`self.FadeInSpeed`)))))
          (if (>= _output_get 1.0)
            (set `self.ScanNormalizedTime` 1.0)
            (`self.UpdateScanState` "NewEnumerator1")))
        (:`NewEnumerator2`
          (bind _output_get_2 (set `self.ScanNormalizedTime` (- (`self.ScanNormalizedTime`) (* (`local.DeltaTime`) (`self.FadeOutSpeed`)))))
          (if (<= _output_get_2 0.0)
            (set `self.ScanNormalizedTime` 0.0)
            (`self.UpdateScanState` "NewEnumerator3")))
        (:`NewEnumerator4`
          (return false)))
      (`KismetMaterialLibrary.SetScalarParameterValue` "/Game/ART/FX/ScanEffect/Scan/Material/MPC_Scan.MPC_Scan" "NormalizedTime" (`self.ScanNormalizedTime`)))
    (:`then_1`
      (return true))))