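; BP_Scan is a scan actor that toggles the far-icon UI on BP_InteractableObject actors through overlap events.
; On begin overlap it clears its CubeSpawned flag, then, for interactables without EyesSpawned, unhides their widget and spawns their far icon.
; On end overlap, if the object's CubeSpanwed flag is set, it removes the icon and marks the object as scanned.
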(event `self.ReceiveActorBeginOverlap`
  (params (OtherActor :type "Actor Object Reference"))
  ;[0 0 0] SpawnCube Ui
  (set `self.CubeSpawned` false)
  (bind _asbp_interactable_object (cast `/Game/GLOBAL/Blueprint/Gameplay/Interaction/BP_InteractableObject` OtherActor))
  (if (not (`/Game/GLOBAL/Blueprint/Gameplay/Interaction/BP_InteractableObject.EyesSpawned` _asbp_interactable_object))
    (`SceneComponent.SetHiddenInGame` (`/Game/GLOBAL/Blueprint/Gameplay/Interaction/BP_InteractableObject.Widget` _asbp_interactable_object) false false)
    (`/Game/GLOBAL/Blueprint/Gameplay/Interaction/BP_InteractableObject.SpawnFarIcon` _asbp_interactable_object)))

(event `self.ReceiveActorEndOverlap`
  (params (OtherActor :type "Actor Object Reference"))
  ;[0 0 0] SpawnCube Ui
  (bind _asbp_interactable_object (cast `/Game/GLOBAL/Blueprint/Gameplay/Interaction/BP_InteractableObject` OtherActor))
  (if (`/Game/GLOBAL/Blueprint/Gameplay/Interaction/BP_InteractableObject.CubeSpanwed` _asbp_interactable_object)
    (`/Game/GLOBAL/Blueprint/Gameplay/Interaction/BP_InteractableObject.UnSpawnFarIcon` _asbp_interactable_object)
    (set `/Game/GLOBAL/Blueprint/Gameplay/Interaction/BP_InteractableObject.Scaned` true _asbp_interactable_object)))

(fn `UserConstructionScript`)