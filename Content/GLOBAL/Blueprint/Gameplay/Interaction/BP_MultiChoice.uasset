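; Interaction actor that displays up to four choices (A to D) through WB_MutliSelect widget components.
; UIManager runs at construction and BeginPlay, passing each choice's struct to CustomizeUI to set text, input, visibility and the open state of the cadena (padlock) image via a material parameter.
; Select, Unselect and Validate events drive only ChoiceA's widget, with selection and deselection also showing or hiding its cadena.
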(event `self.ReceiveBeginPlay`
  (`self.UIManager`))

(event `select`
  (bind _aswb_mutli_select (cast `/Game/GLOBAL/UI/WB_MutliSelect` (`WidgetComponent.GetWidget` (`self.ChoiceA`))))
  (`/Game/GLOBAL/UI/WB_MutliSelect.Select` _aswb_mutli_select)
  (`/Game/GLOBAL/UI/WB_MutliSelect.Display cadena` _aswb_mutli_select))

(event `Unselect`
  (bind _aswb_mutli_select (cast `/Game/GLOBAL/UI/WB_MutliSelect` (`WidgetComponent.GetWidget` (`self.ChoiceA`))))
  (`/Game/GLOBAL/UI/WB_MutliSelect.Unselect` _aswb_mutli_select)
  (`/Game/GLOBAL/UI/WB_MutliSelect.Hide cadena` _aswb_mutli_select))

(event `Validate`
  (bind _aswb_mutli_select (cast `/Game/GLOBAL/UI/WB_MutliSelect` (`WidgetComponent.GetWidget` (`self.ChoiceA`))))
  (`/Game/GLOBAL/UI/WB_MutliSelect.ApplyValidate` _aswb_mutli_select))

(fn `CustomizeUI`
  (params (UI :type "WidgetComponent Object Reference") (Struct :type "/Game/GLOBAL/Blueprint/DATA/S_MultiChoiceCustomize Structure (by ref)"))
  (bind (_event _input _visible_ _opencadena_) (break `/Game/GLOBAL/Blueprint/DATA/S_MultiChoiceCustomize` Struct))
  (bind _aswb_mutli_select (cast `/Game/GLOBAL/UI/WB_MutliSelect` (`WidgetComponent.GetWidget` UI)))
  (`/Game/GLOBAL/UI/WB_MutliSelect.CustomizeTexte` _aswb_mutli_select _event _input)
  (`SceneComponent.SetVisibility` UI _visible_ false)
  (`SceneComponent.SetHiddenInGame` UI (not _visible_) false)
  (bind _returnvalue (`Image.GetDynamicMaterial` (`/Game/GLOBAL/UI/WB_MutliSelect.CadenaImage` _aswb_mutli_select)))
  (`MaterialInstanceDynamic.SetScalarParameterValue` _returnvalue "Offset" (`KismetMathLibrary.SelectFloat` 1.0 0.0 _opencadena_))
  (return))

(fn `UIManager`
  (`self.CustomizeUI` (`self.ChoiceA`) (`self.ChoiceAText`))
  (`self.CustomizeUI` (`self.ChoiceB`) (`self.ChoiceBText`))
  (`self.CustomizeUI` (`self.ChoiceC`) (`self.ChoiceCText`))
  (`self.CustomizeUI` (`self.ChoiceD`) (`self.ChoiceDText`)))

(fn `UserConstructionScript`
  (`self.UIManager`))