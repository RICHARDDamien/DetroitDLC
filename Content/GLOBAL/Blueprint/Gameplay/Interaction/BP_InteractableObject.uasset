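; BP_InteractableObject is an interactable world object that shows a pop-up widget above a configurable static mesh.
; The construction script applies the Mesh variable to TargetMesh, and BeginPlay hides the widget component.
; Spawn and Unspawn events play the matching methods on the WB_PopUp widget.
; Each tick, the widget rotates to face the player camera, acting as a billboard.
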(event `self.ReceiveBeginPlay`
  (`SceneComponent.SetHiddenInGame` (`self.Widget`) true false))

(event `Spawn`
  (`/Game/GLOBAL/UI/WB_PopUp.PlaySpawn` (cast `/Game/GLOBAL/UI/WB_PopUp` (`WidgetComponent.GetWidget` (`self.Widget`)) :!pure true)))

(event `Unspawn`
  (`/Game/GLOBAL/UI/WB_PopUp.PlayUnspawn` (cast `/Game/GLOBAL/UI/WB_PopUp` (`WidgetComponent.GetWidget` (`self.Widget`)) :!pure true)))

(event `self.ReceiveTick`
  (params (DeltaSeconds :type "Float (single-precision)"))
  (bind _widget (`self.Widget`))
  (bind (_returnvalue_location _returnvalue_rotation) (`KismetMathLibrary.BreakTransform` (`KismetAnimationLibrary.K2_LookAt` (`SceneComponent.K2_GetComponentToWorld` _widget) (`self.K2_GetActorLocation` (`GameplayStatics.GetPlayerCameraManager` 0)) (1.0 0.0 0.0) true (0.0 0.0 1.0))))
  (`SceneComponent.K2_SetWorldRotation` _widget _returnvalue_rotation false false))

(fn `UserConstructionScript`
  (`StaticMeshComponent.SetStaticMesh` (`self.TargetMesh`) (`self.Mesh`)))