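; BP_DisplayMission is an actor that shows mission text through two widget components: a text widget and a background panel.
; Configurable texts and offsets are pushed into both widgets at construction and BeginPlay, when both components are also hidden.
; The player pawn entering the Box trigger reveals them once and runs their spawn functions.
; Spawn can also be called directly, while Unspawn runs the widgets' unspawn functions and hides them after one second.
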(event `self.ReceiveBeginPlay`
  (`SceneComponent.SetHiddenInGame` (`self.BackGround`) true false)
  (`SceneComponent.SetHiddenInGame` (`self.Texte`) true false)
  (`self.SetUItext`))

(event `Spawn`
  (bind _texte (`self.Texte`))
  (`SceneComponent.SetHiddenInGame` _texte false false :!label _label)
  (`SceneComponent.SetHiddenInGame` (`self.BackGround`) false false)
  (bind _aswb_mission_text (cast `/Game/GLOBAL/UI/WB_MissionText` (`WidgetComponent.GetWidget` _texte)))
  (bind _aswb_global_mission_panel (cast `/Game/GLOBAL/UI/WB_GlobalMissionPanel` (`WidgetComponent.GetWidget` (`self.BackGround`))))
  (`/Game/GLOBAL/UI/WB_MissionText.SpawnUI` _aswb_mission_text)
  (`/Game/GLOBAL/UI/WB_GlobalMissionPanel.Spawn` _aswb_global_mission_panel))

(event `self.Box.OnComponentBeginOverlap`
  (params (OverlappedComponent :type "PrimitiveComponent Object Reference") (OtherActor :type "Actor Object Reference") (OtherComp :type "PrimitiveComponent Object Reference") (OtherBodyIndex :type Integer) (bFromSweep :type Boolean) (SweepResult :type "HitResult Structure (by ref)"))
  (if (== OtherActor (`GameplayStatics.GetPlayerPawn` 0))
    (`/Engine/EditorBlueprintResources/StandardMacros.DoOnce` false
      (:`Completed`
        (goto _label)))))

(event `Unspawn`
  (bind _aswb_mission_text (cast `/Game/GLOBAL/UI/WB_MissionText` (`WidgetComponent.GetWidget` (`self.Texte`))))
  (bind _aswb_global_mission_panel (cast `/Game/GLOBAL/UI/WB_GlobalMissionPanel` (`WidgetComponent.GetWidget` (`self.BackGround`))))
  (`/Game/GLOBAL/UI/WB_MissionText.Unspawn` _aswb_mission_text)
  (`/Game/GLOBAL/UI/WB_GlobalMissionPanel.Unspawn` _aswb_global_mission_panel)
  (`KismetSystemLibrary.Delay` 1.0)
  (`SceneComponent.SetHiddenInGame` (`self.BackGround`) true false)
  (`SceneComponent.SetHiddenInGame` (`self.Texte`) true false))

(fn `SetUItext`
  (bind _bigtexte (`self.BigTexte`))
  (bind _small_text (`self.Small Text`))
  (bind _small_text_offset (`self.Small Text Offset`))
  (bind _big_text_offset (`self.Big Text Offset`))
  (bind _aswb_mission_text (cast `/Game/GLOBAL/UI/WB_MissionText` (`WidgetComponent.GetWidget` (`self.Texte`))))
  (`/Game/GLOBAL/UI/WB_MissionText.ApplyNewTexte` _aswb_mission_text _bigtexte _small_text _small_text_offset _big_text_offset)
  (bind _aswb_global_mission_panel (cast `/Game/GLOBAL/UI/WB_GlobalMissionPanel` (`WidgetComponent.GetWidget` (`self.BackGround`))))
  (`/Game/GLOBAL/UI/WB_MissionText.ApplyNewTexte` (`/Game/GLOBAL/UI/WB_GlobalMissionPanel.WB_MissionText` _aswb_global_mission_panel) _bigtexte _small_text _small_text_offset _big_text_offset))

(fn `UserConstructionScript`
  (`self.SetUItext`))